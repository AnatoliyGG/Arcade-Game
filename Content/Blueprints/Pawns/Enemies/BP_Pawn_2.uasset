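; Enemy pawn that moves continuously and steers in yaw to home in on the player pawn cached at BeginPlay.
; Each tick it moves a fixed, unswept step along local -X, independent of delta time.
; It turns by the current-minus-look-at yaw difference, clamped to RotMaxSpeed and scaled by delta time, swinging its -X travel direction toward the player.
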(event EventBeginPlay
  (|CallParentFunction)
  (Variables|Default|SetPlayerPawn (Game|Player|GetPlayerPawn 0)))

(event EventTick
  (params (DeltaSeconds :type Float%20%28single-precision%29))
  (bind _rot_max_speed (Variables|Default|GetRot%20Max%20Speed))
  (|CallParentFunction DeltaSeconds)
  (Transformation|AddActorLocalOffset "-3.000000, 0, 0" false false)
  (Variables|Default|GetPlayerPawn
    (:then
      (Transformation|AddActorLocalRotation (Math|Rotator|MakeRotator 0.0 0.0 (* (Math|Float|Clamp(Float) (.yaw (Math|Rotator|Delta(Rotator) (Transformation|GetActorRotation) (Math|Rotator|FindLookatRotation (Transformation|GetActorLocation) (Transformation|GetActorLocation (Variables|Default|GetPlayerPawn))))) (* -1.0 _rot_max_speed) _rot_max_speed) (Utilities|Time|GetWorldDeltaSeconds))) false false))
    (:else)))

(fn ConstructionScript)